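; BP_Test is a homework test Blueprint that demonstrates basic arithmetic and branching with on-screen debug text.
; On BeginPlay it prints the sum, difference, product and quotient of NumA and NumB via formatted text, all labelled "Add Number".
; It then compares the quotient to NumC and prints whether it is higher or smaller, with equality counting as higher.
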(event EventBeginPlay
  (bind _numb (Variables|Default|GetNumB))
  (bind _numa (Variables|Default|GetNumA))
  (bind _returnvalue (/ _numa _numb))
  ;[1 0.1765 0.1666] Add
  (Development|PrintString (Utilities|String|ToString(Text) (Utilities|Text|FormatText "Add Number {1} + {2} = {3}" (Variables|Default|GetNumA) (Variables|Default|GetNumB) (+ (Variables|Default|GetNumA) (Variables|Default|GetNumB)))) true true "(R=0.000000,G=0.660000,B=1.000000,A=1.000000)" (Variables|Default|GetShowTime))
  ;[0.165 0.3104 1] Subtract
  (Development|PrintString (Utilities|String|ToString(Text) (Utilities|Text|FormatText "Add Number {1} - {2} = {3}" (Variables|Default|GetNumA) (Variables|Default|GetNumB) (- (Variables|Default|GetNumA) (Variables|Default|GetNumB)))) true true "(R=0.000000,G=0.660000,B=1.000000,A=1.000000)" (Variables|Default|GetShowTime))
  ;[0.2871 1 0.2816] Multiply
  (Development|PrintString (Utilities|String|ToString(Text) (Utilities|Text|FormatText "Add Number {1} * {2} = {3}" (Variables|Default|GetNumA) (Variables|Default|GetNumB) (* (Variables|Default|GetNumA) (Variables|Default|GetNumB)))) true true "(R=0.000000,G=0.660000,B=1.000000,A=1.000000)" (Variables|Default|GetShowTime))
  ;[1 0.8137 0.2266] Divide
  (Development|PrintString (Utilities|String|ToString(Text) (Utilities|Text|FormatText "Add Number {1} / {2} = {3}" (Variables|Default|GetNumA) (Variables|Default|GetNumB) _returnvalue)) true true "(R=0.000000,G=0.660000,B=1.000000,A=1.000000)" (Variables|Default|GetShowTime))
  ;[1 0.07855 0.8048] Branch
  (if (>= _returnvalue (Variables|Default|GetNumC))
    (Development|PrintString "Higher than NumC!" true true "(R=0.000000,G=0.660000,B=1.000000,A=1.000000)" (Variables|Default|GetShowTime))
    (else
      (Development|PrintString "Smaller than NumC!" true true "(R=0.000000,G=0.660000,B=1.000000,A=1.000000)" (Variables|Default|GetShowTime)))))

(event Collision|EventActorBeginOverlap
  (params (OtherActor :type Actor%20Object%20Reference)))

(event EventTick
  (params (DeltaSeconds :type Float%20%28single-precision%29)))

(fn ConstructionScript)