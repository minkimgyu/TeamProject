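; BP_Knut is a monster character that wanders between four set locations and chases the player.
; Roaming walks it slowly through randomly branching chains of AIMoveTo calls over those points.
; When PawnSensing sees a pawn, it speeds up toward player 0, and a one-second retriggerable delay resumes roaming once sightings stop.
; The perception handler is empty; the run-and-attack montage loop is never triggered here, and older movement experiments sit disconnected.
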(event OnSeePawn(PawnSensing)
  (params (Pawn :type Pawn%20Object%20Reference))
  ;[1 1 1] AI 랜덤 좌표 배회 및 탐지 추적
  (Utilities|FlowControl|Sequence
    (:then_0
      (Variables|/Script/Engine.CharacterMovementComponent|SetMaxWalkSpeed (Variables|Character|GetCharacterMovement) 5e+02)
      (AI|AIMoveTo self "0, 0, 0" (Game|GetPlayerCharacter 0) 5.0 false))
    (:then_1
      (Utilities|FlowControl|RetriggerableDelay 1.0)
      (CallFunction|Roaming))))

(event OnTargetPerceptionUpdated(AIPerception)
  (params (Actor :type Actor%20Object%20Reference) (Stimulus :type AI%20Stimulus%20Structure))
  ;[1 1 1] AI Noise Perception
)

(event Custom|RunToPlayer
  ;[1 1 1] 사용 안함
  (AI|AIMoveTo self "0, 0, 0" (Game|GetPlayerController 0) 4e+01 false
    (:OnSuccess
      (CallFunction|AttackPlayer))
    (:OnFail
      (CallFunction|RuntoPlayer))))

(event Custom|AttackPlayer
  ;[1 1 1] 사용 안함
  (Animation|Montage|PlayMontage (Variables|Character|GetMesh) 0 1.5
    (:OnCompleted
      (CallFunction|RuntoPlayer))))

(event Custom|Roaming
  (bind _self self)
  ;[1 1 1] AI 랜덤 좌표 배회 및 탐지 추적
  (Variables|/Script/Engine.CharacterMovementComponent|SetMaxWalkSpeed (Variables|Character|GetCharacterMovement) 2e+02)
  ;[1 1 1] 특정 좌표 랜덤 배회
  (switch int (Math|Random|RandomIntegerinRange 0 3)
    (:0
      (AI|AIMoveTo _self (Variables|Default|GetLocation%201) 0 5.0 false :!label _label
        (:OnSuccess
          (switch int (Math|Random|RandomIntegerinRange 0 1)
            (:0
              (AI|AIMoveTo _self (Variables|Default|GetLocation%202) 0 5.0 false
                (:OnSuccess
                  (goto _label))))
            (:1
              (AI|AIMoveTo _self (Variables|Default|GetLocation%204) 0 5.0 false
                (:OnSuccess
                  (AI|AIMoveTo _self (Variables|Default|GetLocation%203) 0 5.0 false :!label _label_2
                    (:OnSuccess
                      (switch int (Math|Random|RandomIntegerinRange 0 1)
                        (:0
                          (AI|AIMoveTo _self (Variables|Default|GetLocation%202) 0 5.0 false
                            (:OnSuccess
                              (goto _label_2))))
                        (:1
                          (AI|AIMoveTo _self (Variables|Default|GetLocation%204) 0 5.0 false
                            (:OnSuccess
                              (goto _label))))))))))))))
    (:1
      (AI|AIMoveTo _self (Variables|Default|GetLocation%202) 0 5.0 false :!label _label_3
        (:OnSuccess
          (switch int (Math|Random|RandomIntegerinRange 0 1)
            (:0
              (AI|AIMoveTo _self (Variables|Default|GetLocation%203) 0 5.0 false
                (:OnSuccess
                  (goto _label_3))))
            (:1
              (AI|AIMoveTo _self (Variables|Default|GetLocation%201) 0 5.0 false
                (:OnSuccess
                  (AI|AIMoveTo _self (Variables|Default|GetLocation%204) 0 5.0 false :!label _label_4
                    (:OnSuccess
                      (switch int (Math|Random|RandomIntegerinRange 0 1)
                        (:0
                          (AI|AIMoveTo _self (Variables|Default|GetLocation%203) 0 5.0 false
                            (:OnSuccess
                              (goto _label_3))))
                        (:1
                          (AI|AIMoveTo _self (Variables|Default|GetLocation%201) 0 5.0 false
                            (:OnSuccess
                              (goto _label_4))))))))))))))
    (:2
      (goto _label_2))
    (:3
      (goto _label_4))))

(event EventBeginPlay
  ;[1 1 1] AI 랜덤 좌표 배회 및 탐지 추적
  (CallFunction|Roaming))

(fn ConstructionScript)