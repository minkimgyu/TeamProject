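; Knut monster AI that roams randomly between four set locations, investigates the player's perceived stimuli and speeds up to chase when it sees a pawn.
; Chained AIMoveTo calls drive movement, with a retriggerable delay returning it to roaming after sight events stop.
; Each tick, it fans Visibility line traces across a view angle and rebuilds procedural mesh sections from the results as a field-of-view display, separate from detection.
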(event OnSeePawn(PawnSensing)
  (params (Pawn :type Pawn%20Object%20Reference))
  ;[1 1 1] AI 랜덤 좌표 배회 및 탐지 추적
  (Utilities|FlowControl|Sequence
    (:then_0
      (Variables|/Script/Engine.CharacterMovementComponent|SetMaxWalkSpeed (Variables|Character|GetCharacterMovement) 5e+02)
      (AI|AIMoveTo self "0, 0, 0" (Game|GetPlayerCharacter 0) 5.0 false))
    (:then_1
      (Utilities|FlowControl|RetriggerableDelay 1.0)
      (CallFunction|Roaming))))

(event OnTargetPerceptionUpdated(AIPerception)
  (params (Actor :type Actor%20Object%20Reference) (Stimulus :type AI%20Stimulus%20Structure))
  (bind (_age _expirationage _strength _stimuluslocation _receiverlocation _tag _bsuccessfullysensed) (Utilities|Struct|BreakAIStimulus Stimulus))
  ;[1 1 1] AI Noise Perception
  (Utilities|Casting|CastToBP_FirstPersonCharacter Actor)
  (if _bsuccessfullysensed
    (Variables|Default|SetInvestigating? true)
    (AI|AIMoveTo self _stimuluslocation 0 5.0 false
      (:OnSuccess
        (Utilities|FlowControl|Delay 1.0)
        (CallFunction|Roaming)))))

(event Custom|RunToPlayer
  ;[1 1 1] 사용 안함
  (AI|AIMoveTo self "0, 0, 0" (Game|GetPlayerController 0) 4e+01 false
    (:OnSuccess
      (CallFunction|AttackPlayer))
    (:OnFail
      (CallFunction|RuntoPlayer))))

(event Custom|AttackPlayer
  ;[1 1 1] 사용 안함
  (Animation|Montage|PlayMontage (Variables|Character|GetMesh) 0 1.5
    (:OnCompleted
      (CallFunction|RuntoPlayer))))

(event Custom|Roaming
  (bind _self self)
  ;[1 1 1] AI 랜덤 좌표 배회 및 탐지 추적
  (Variables|/Script/Engine.CharacterMovementComponent|SetMaxWalkSpeed (Variables|Character|GetCharacterMovement) 2e+02)
  ;[1 1 1] 특정 좌표 랜덤 배회
  (switch int (Math|Random|RandomIntegerinRange 0 3)
    (:0
      (AI|AIMoveTo _self (Variables|Default|GetLocation%201) 0 5.0 false :!label _label
        (:OnSuccess
          (switch int (Math|Random|RandomIntegerinRange 0 1)
            (:0
              (AI|AIMoveTo _self (Variables|Default|GetLocation%202) 0 5.0 false
                (:OnSuccess
                  (goto _label))))
            (:1
              (AI|AIMoveTo _self (Variables|Default|GetLocation%204) 0 5.0 false
                (:OnSuccess
                  (AI|AIMoveTo _self (Variables|Default|GetLocation%203) 0 5.0 false :!label _label_2
                    (:OnSuccess
                      (switch int (Math|Random|RandomIntegerinRange 0 1)
                        (:0
                          (AI|AIMoveTo _self (Variables|Default|GetLocation%202) 0 5.0 false
                            (:OnSuccess
                              (goto _label_2))))
                        (:1
                          (AI|AIMoveTo _self (Variables|Default|GetLocation%204) 0 5.0 false
                            (:OnSuccess
                              (goto _label))))))))))))))
    (:1
      (AI|AIMoveTo _self (Variables|Default|GetLocation%202) 0 5.0 false :!label _label_3
        (:OnSuccess
          (switch int (Math|Random|RandomIntegerinRange 0 1)
            (:0
              (AI|AIMoveTo _self (Variables|Default|GetLocation%203) 0 5.0 false
                (:OnSuccess
                  (goto _label_3))))
            (:1
              (AI|AIMoveTo _self (Variables|Default|GetLocation%201) 0 5.0 false
                (:OnSuccess
                  (AI|AIMoveTo _self (Variables|Default|GetLocation%204) 0 5.0 false :!label _label_4
                    (:OnSuccess
                      (switch int (Math|Random|RandomIntegerinRange 0 1)
                        (:0
                          (AI|AIMoveTo _self (Variables|Default|GetLocation%203) 0 5.0 false
                            (:OnSuccess
                              (goto _label_3))))
                        (:1
                          (AI|AIMoveTo _self (Variables|Default|GetLocation%201) 0 5.0 false
                            (:OnSuccess
                              (goto _label_4))))))))))))))
    (:2
      (goto _label_2))
    (:3
      (goto _label_4))))

(event EventBeginPlay
  ;[1 1 1] AI 랜덤 좌표 배회 및 탐지 추적
  (CallFunction|Roaming))

(event EventTick
  (params (DeltaSeconds :type Float%20%28single-precision%29))
  (CallFunction|Update)
  (CallFunction|LineTracing))

(fn ConstructionScript
  (if (Variables|FieldOfVision|Debug|GetbRebuild)
    _
    (else
      _))
  (CallFunction|Start)
  (CallFunction|LineTracing))

(fn Start
  (Utilities|FlowControl|Sequence
    (:then_0
      (bind _output_get (Variables|FieldOfVision|Auxiliary|SetNumberOfSections (Math|Float|Ceil (/ (* (Variables|FieldOfVision|Base|GetHalfAngle) 2.0) (Variables|FieldOfVision|Base|GetDeltaAngle)))))
      (Variables|FieldOfVision|Auxiliary|SetdAngle (/ (* (Variables|FieldOfVision|Base|GetHalfAngle) 2.0) _output_get)))
    (:then_1
      (Variables|FieldOfVision|Auxiliary|SetStartPoint (+ (Math|Vector|MakeVector 0.0 0.0 (- (Variables|FieldOfVision|Base|GetHeightOfCheck) 1e+02)) (Transformation|GetActorLocation))))
    (:then_2
      (Transformation|AddLocalOffset (Variables|Default|GetProceduralMesh) (Math|Vector|MakeVector 0.0 0.0 (- (Variables|FieldOfVision|Base|GetHeightOfShow) 1e+02)) false false))))

(fn LineTracing
  (bind _startpoint (Variables|FieldOfVision|Auxiliary|GetStartPoint))
  (for _index (range 0 (Variables|FieldOfVision|Auxiliary|GetNumberOfSections))
    (LocalVariables|SetL_CurrentAngle (- (* _index (Variables|FieldOfVision|Auxiliary|GetdAngle)) (Variables|FieldOfVision|Base|GetHalfAngle)))
    (bind _outhit (Collision|LineTraceByChannel _startpoint (+ _startpoint (* (Math|Vector|RotateVectorAroundAxis (Transformation|GetActorForwardVector) (LocalVariables|GetL_CurrentAngle) "0.000000,0.000000,1.000000") (Variables|FieldOfVision|Base|GetExternalRadius))) "TraceTypeQuery1" false 0 (Variables|FieldOfVision|Debug|GetDraw%20Debug%20Type) true "(R=1.000000,G=0.000000,B=0.000000,A=1.000000)" "(R=0.000000,G=1.000000,B=0.000000,A=1.000000)" (Variables|FieldOfVision|Debug|GetDraw%20Debug%20Time)))
    (Utilities|Array|Add (Variables|Default|GetHitResults) _outhit))
  (CallFunction|CreateProceduralMesh))

(fn CreateProceduralMesh
  (for _index (range 0 (- (Utilities|Array|LastIndex (Variables|Default|GetHitResults)) 0))
    (LocalVariables|Seti _index)
    (Utilities|FlowControl|Sequence
      (:then_0
        (if (.bBlockingHit (Collision|BreakHitResult (Utilities|Array|Get(acopy) (Variables|Default|GetHitResults) (LocalVariables|Geti))))
          (LocalVariables|SetL_LeftPoint (.Location (Collision|BreakHitResult (Utilities|Array|Get(acopy) (Variables|Default|GetHitResults) (LocalVariables|Geti)))))
          (else
            (LocalVariables|SetL_LeftPoint (.TraceEnd (Collision|BreakHitResult (Utilities|Array|Get(acopy) (Variables|Default|GetHitResults) (LocalVariables|Geti))))))))
      (:then_1
        (if (.bBlockingHit (Collision|BreakHitResult (Utilities|Array|Get(acopy) (Variables|Default|GetHitResults) (+ (LocalVariables|Geti) 0))))
          (LocalVariables|SetL_RightPoint (.Location (Collision|BreakHitResult (Utilities|Array|Get(acopy) (Variables|Default|GetHitResults) (+ (LocalVariables|Geti) 0)))))
          (else
            (LocalVariables|SetL_RightPoint (.TraceEnd (Collision|BreakHitResult (Utilities|Array|Get(acopy) (Variables|Default|GetHitResults) (+ (LocalVariables|Geti) 0))))))))
      (:then_2
        (Class|ProceduralMeshComponent|CreateMeshSectionLinearColor (Variables|Default|GetProceduralMesh) (LocalVariables|Geti) (Utilities|Array|MakeArray (- (Variables|FieldOfVision|Auxiliary|GetStartPoint) (Variables|FieldOfVision|Auxiliary|GetStartPoint)) (- (LocalVariables|GetL_LeftPoint) (Variables|FieldOfVision|Auxiliary|GetStartPoint)) (- (LocalVariables|GetL_RightPoint) (Variables|FieldOfVision|Auxiliary|GetStartPoint))) (Utilities|Array|MakeArray 0 2 1) 0 0 0 0 0 0 0 false false)
        (Rendering|Material|SetMaterial (Variables|Default|GetProceduralMesh) (LocalVariables|Geti) "/Game/_Main/Monster/Materials/MI_Base.MI_Base"))))
  (Transformation|SetRelativeRotation (Variables|Default|GetProceduralMesh) (* (Math|Rotator|MakeRotfromX (Transformation|GetActorForwardVector)) -1.0) false false))

(fn Update
  (Variables|FieldOfVision|Auxiliary|SetStartPoint (+ (Math|Vector|MakeVector 0.0 0.0 (- (Variables|FieldOfVision|Base|GetHeightOfCheck) 1e+02)) (Transformation|GetActorLocation)))
  (Utilities|Array|Clear (Variables|Default|GetHitResults))
  (Class|ProceduralMeshComponent|ClearAllMeshSections (Variables|Default|GetProceduralMesh)))