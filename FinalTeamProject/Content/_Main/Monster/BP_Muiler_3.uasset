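; Muiler monster enemy that guards a fixed spot, investigates noises, chases the seen player and damages whatever its capsule hits.
; AI Perception sends it to noises; PawnSensing starts pursuit and GM_Main's chase effect, with a retriggerable delay ending both.
; Point damage always stuns it briefly, since Health is compared to itself.
; Roaming just returns to Location1 and turns; random patrols are disconnected and the montage attack loop is unused.
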(event OnSeePawn(PawnSensing)
  (params (Pawn :type Pawn%20Object%20Reference))
  (bind _gm_main (Variables|Default|GetGM%20Main))
  ;[1 1 1] AI 랜덤 좌표 배회 및 탐지 추적
  (Utilities|FlowControl|Sequence
    (:then_0
      (Variables|/Script/Engine.CharacterMovementComponent|SetMaxWalkSpeed (Variables|Character|GetCharacterMovement) 2e+02)
      (AI|AIMoveTo self "0, 0, 0" (Game|GetPlayerCharacter 0) 5.0 false))
    (:then_1
      (Utilities|FlowControl|RetriggerableDelay 1.0)
      (CallFunction|Roaming)
      (Default|EndChasing _gm_main)
      (Variables|Default|SetNowChase false))
    (:then_2
      (if (not (Variables|Default|GetNowChase))
        (Variables|Default|SetNowChase true)
        (Default|ChasingEffect _gm_main)))))

(event OnTargetPerceptionUpdated(AIPerception)
  (params (Actor :type Actor%20Object%20Reference) (Stimulus :type AI%20Stimulus%20Structure))
  (bind (_age _expirationage _strength _stimuluslocation _receiverlocation _tag _bsuccessfullysensed) (Utilities|Struct|BreakAIStimulus Stimulus))
  ;[1 1 1] AI Noise Perception
  (Utilities|Casting|CastToBP_FirstPersonCharacter Actor)
  (if _bsuccessfullysensed
    (Variables|Default|SetInvestigating? true)
    (AI|AIMoveTo self _stimuluslocation 0 5.0 false
      (:OnSuccess
        (Utilities|FlowControl|Delay 1.0)
        (CallFunction|Roaming)))))

(event OnComponentHit(CapsuleComponent)
  (params (HitComponent :type Primitive%20Component%20Object%20Reference) (OtherActor :type Actor%20Object%20Reference) (OtherComp :type Primitive%20Component%20Object%20Reference) (NormalImpulse :type Vector :default "0, 0, 0") (Hit :type Hit%20Result%20Structure%20%28by%20ref%29))
  (Game|Damage|ApplyDamage OtherActor 2e+01 0 self))

(event Custom|RunToPlayer
  ;[1 1 1] 사용 안함
  (AI|AIMoveTo self "0, 0, 0" (Game|GetPlayerController 0) 4e+01 false
    (:OnSuccess
      (CallFunction|AttackPlayer))
    (:OnFail
      (CallFunction|RuntoPlayer))))

(event Custom|AttackPlayer
  ;[1 1 1] 사용 안함
  (Animation|Montage|PlayMontage (Variables|Character|GetMesh) 0 1.5
    (:OnCompleted
      (CallFunction|RuntoPlayer))))

(event Custom|Roaming
  ;[1 1 1] AI 랜덤 좌표 배회 및 탐지 추적
  (Variables|/Script/Engine.CharacterMovementComponent|SetMaxWalkSpeed (Variables|Character|GetCharacterMovement) 2e+02)
  ;[1 1 1] 제자리
  (AI|AIMoveTo self (Variables|Default|GetLocation%201) 0 5.0 false
    (:OnSuccess
      (Transformation|SetActorRotation "0.000000,-180.000000,0.000000"))))

(event Custom|Stun
  ;[1 1 1] 데미지 받을시 스턴
  (Variables|Default|SetIsHit? true)
  (Pawn|Components|CharacterMovement|DisableMovement (Variables|Character|GetCharacterMovement))
  (Utilities|FlowControl|Delay 5.0)
  (Pawn|Components|CharacterMovement|SetMovementMode (Variables|Character|GetCharacterMovement) "MOVE_Walking" 0))

(event EventBeginPlay
  ;[1 1 1] AI 랜덤 좌표 배회 및 탐지 추적
  (Utilities|FlowControl|Sequence
    (:then_0
      (CallFunction|Roaming))
    (:then_1
      (bind _asgm_main (Utilities|Casting|CastToGM_Main (Game|GetGameMode)))
      (Variables|Default|SetGM%20Main _asgm_main))))

(event Game|Damage|EventPointDamage
  (params (Damage :type Float%20%28single-precision%29) (DamageType :type Damage%20Type%20Object%20Reference) (HitLocation :type Vector :default "0, 0, 0") (HitNormal :type Vector :default "0, 0, 0") (HitComponent :type Primitive%20Component%20Object%20Reference) (BoneName :type Name :default "None") (ShotFromDirection :type Vector :default "0, 0, 0") (InstigatedBy :type Controller%20Object%20Reference) (DamageCauser :type Actor%20Object%20Reference) (HitInfo :type Hit%20Result%20Structure%20%28by%20ref%29))
  ;[1 1 1] 데미지 받을시 스턴
  (if (<= (Variables|Default|GetHealth) (Variables|Default|GetHealth))
    (CallFunction|Stun)
    (else
      (Variables|Default|SetHealth (- (Variables|Default|GetHealth) Damage)))))

(fn ConstructionScript)