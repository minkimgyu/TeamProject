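; BP_TestInteractionActor is a test interactable actor with a cube and a point light, driven by interaction interface events.
; Focus changes toggle custom depth rendering on the cube.
; Each interact flips a boolean that shows or hides the point light.
; The trace reset event is left empty, as are BeginPlay, Tick and the construction script.
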(event EventBeginPlay)

(event Collision|EventActorBeginOverlap
  (params (OtherActor :type Actor%20Object%20Reference)))

(event EventTick
  (params (DeltaSeconds :type Float%20%28single-precision%29)))

(event EventInterfaceToggleFocus
  (params (Focus :type Boolean))
  (Rendering|SetRenderCustomDepth (Variables|Default|GetCube) Focus))

(event EventInterfaceInteract
  (bind _pointlight (Variables|Default|GetPointLight))
  (Variables|Default|SetInteractToggle (not (Variables|Default|GetInteractToggle)))
  (if (Variables|Default|GetInteractToggle)
    (Rendering|SetVisibility _pointlight true false)
    (else
      (Rendering|SetVisibility _pointlight false false))))

(event EventResetInteractionTrace)

(fn ConstructionScript)