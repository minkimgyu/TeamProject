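; BP_ExitDoor is an interactable exit door that starts locked and can only be used once it has been unlocked.
; OpenDoor clears the lock, swaps the Korean prompt from locked to press-E, sets the open outline and plays a key sound.
; Interacting calls InteractWithDoor only when unlocked.
; Focus toggles custom depth on the door mesh, with GMMain setting the lock or open outline style to match its state.
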(event Custom|OpenDoor
  (Variables|Default|SetNowLocked false)
  (Default|SetTxt (Variables|Default|GetWB%20Interaction%202) "E를 눌러 탈출구 문을 엽니다.")
  (Default|SetOpenOutline (Variables|Default|GetGM%20Main))
  (Audio|PlaySoundatLocation "/Game/_Main/Sound/Key/key.key" (Transformation|GetWorldLocation (Variables|Default|GetCube3)) "0, 0, 0" 1.0 1.0 0.0 0 0 0 0))

(event EventBeginPlay
  (CallFunction|Init)
  (Default|SetTxt (Variables|Default|GetWB%20Interaction%202) "탈출구 문이 잠겨있습니다.")
  (Variables|Default|SetNowLocked true))

(event Collision|EventActorBeginOverlap
  (params (OtherActor :type Actor%20Object%20Reference))
  (|CallParentFunction OtherActor) ; This node is disabled and will not be called.\nDrag off pins to build functionality.
)

(event EventTick
  (params (DeltaSeconds :type Float%20%28single-precision%29))
  (|CallParentFunction DeltaSeconds) ; This node is disabled and will not be called.\nDrag off pins to build functionality.
)

(event EventInterfaceToggleFocus
  (params (Focus :type Boolean))
  (bind _gm_main (Variables|Default|GetGM%20Main))
  (if Focus
    (if (Variables|Default|GetNowLocked)
      (Default|SetLockOutline _gm_main)
      (else
        (Default|SetOpenOutline _gm_main)))
    (else
      (Default|SetOpenOutline (Variables|Default|GetGM%20Main))))
  (Rendering|SetRenderCustomDepth (Variables|Default|GetDoor) Focus))

(event EventInterfaceInteract
  (if (not (Variables|Default|GetNowLocked))
    (CallFunction|InteractwithDoor)))

(fn ConstructionScript
  (|CallParentFunction))