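; BP_PortalToClear is an exit portal that ends the game once the player meets the clear condition.
; When the first-person character enters its box, it calls CheckClearGame on the character's inventory system.
; If that passes, it stores the start menu as the next scene in the GI_Instance game instance and opens the loading screen level, handing the destination through the game instance.
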(event OnComponentBeginOverlap(Box)
  (params (OverlappedComponent :type Primitive%20Component%20Object%20Reference) (OtherActor :type Actor%20Object%20Reference) (OtherComp :type Primitive%20Component%20Object%20Reference) (OtherBodyIndex :type Integer) (bFromSweep :type Boolean) (SweepResult :type Hit%20Result%20Structure%20%28by%20ref%29))
  (bind _asbp_first_person_character (Utilities|Casting|CastToBP_FirstPersonCharacter OtherActor))
  (bind _canclear (Default|CheckClearGame (Variables|/Game/Collaboration/Kim/FirstPerson/Blueprints/BP_FirstPersonCharacter.BP_FirstPersonCharacter_C|GetInventorySystem _asbp_first_person_character)))
  (if _canclear
    (bind _asgi_instance (Utilities|Casting|CastToGI_Instance (Game|GetGameInstance)))
    (Variables|/Game/FirstPerson/test/GI_Instance.GI_Instance_C|SetInsNextSceneName _asgi_instance "startmenu")
    (Game|OpenLevel(byName) " loadingscreen")))

(event Collision|EventActorBeginOverlap
  (params (OtherActor :type Actor%20Object%20Reference))
  (|CallParentFunction OtherActor) ; This node is disabled and will not be called.\nDrag off pins to build functionality.
)

(event EventTick
  (params (DeltaSeconds :type Float%20%28single-precision%29))
  (|CallParentFunction DeltaSeconds) ; This node is disabled and will not be called.\nDrag off pins to build functionality.
)

(fn ConstructionScript
  (|CallParentFunction))