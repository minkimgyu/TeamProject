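; Actor component on the first-person character that finds what the player is looking at and routes interaction to it.
; Each tick a camera line trace updates the focused actor and toggles highlight on interaction areas that allow focus.
; The controller's interact event messages the focused actor's ItemDataComponent, or the actor itself if it has none.
; A separate TryToInteract event messages the parent actor of the focused interaction area.
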(event Custom|InteractWithItem
  (bind _bp_first_person_character (Variables|Default|GetBP%20First%20Person%20Character))
  (bind _ac_interactiontrace (Variables|/Game/Collaboration/Kim/FirstPerson/Blueprints/BP_FirstPersonCharacter.BP_FirstPersonCharacter_C|GetAC_InteractionTrace _bp_first_person_character))
  (bind _focusedactor (Variables|AC_InteractionTrace_C|GetFocusedActor _ac_interactiontrace))
  (bind _returnvalue (Actor|GetComponentbyClass _focusedactor "/Game/Collaboration/Kim/Inventory/ItemDataComponent.ItemDataComponent_C"))
  (Utilities|IsValid _focusedactor
    (:Is%20Valid
      (Utilities|IsValid _returnvalue
        (:Is%20Valid
          (Class|IInteractInterface|Interactwith(Message) _returnvalue (Variables|Default|GetBP%20First%20Person%20Character)))
        (:Is%20Not%20Valid
          (Class|IInteractInterface|Interactwith(Message) _focusedactor (Variables|Default|GetBP%20First%20Person%20Character)))))
    (:Is%20Not%20Valid
      (Development|PrintString "This is box"))))

(event Custom|TryToInteract
  (params (in :type Boolean))
  (if in
    (if (Variables|Default|GetIsTracingInteracionArea)
      (Class|BIInteraction|InterfaceInteract(Message) (Actor|GetParentActor (Variables|Default|GetFocusedInteractionArea))))))

(event EventBeginPlay
  (Utilities|FlowControl|Sequence
    (:then_0
      (bind _asbp_controller (Utilities|Casting|CastToBP_Controller (Game|GetPlayerController 0)))
      (Variables|Default|SetBP%20Controller _asbp_controller))
    (:then_1
      (bind _asbp_first_person_character (Utilities|Casting|CastToBP_FirstPersonCharacter (Components|GetOwner)))
      (Variables|Default|SetBP%20First%20Person%20Character _asbp_first_person_character))
    (:then_2
      (EventDispatchers|BindEventtoInteract (Variables|Default|GetBP%20Controller) (delegate Custom|InteractWithItem)))))

(event EventTick
  (params (DeltaSeconds :type Float%20%28single-precision%29))
  (CallFunction|Trace))

(fn Trace
  (bind _returnvalue (Game|GetPlayerCameraManager 0))
  (bind _returnvalue_2 (Transformation|GetActorLocation _returnvalue))
  (bind (_outhit _returnvalue_3) (Collision|LineTraceByChannel _returnvalue_2 (+ _returnvalue_2 (* (Math|Vector|GetForwardVector (Transformation|GetActorRotation _returnvalue)) (Variables|Default|GetLength))) "TraceTypeQuery2" false 0 "None"))
  (if _returnvalue_3
    (if (!= (Variables|Default|GetFocusedActor) (.HitActor (Collision|BreakHitResult _outhit)))
      (Variables|Default|SetFocusedActor (.HitActor (Collision|BreakHitResult _outhit)))
      (CallFunction|TraceInteractionArea (or (== (Utilities|GetClass (.HitActor (Collision|BreakHitResult _outhit))) "/Game/Collaboration/Kim/Interaction/InteractionArea/BP_InteractionArea_Box.BP_InteractionArea_Box_C") (== (Utilities|GetClass (.HitActor (Collision|BreakHitResult _outhit))) "/Game/Collaboration/Kim/Interaction/InteractionArea/BP_InteractionArea_CustomShape.BP_InteractionArea_CustomShape_C"))))
    (else
      (Variables|Default|SetFocusedActor 0)
      (CallFunction|TraceInteractionArea false))))

(fn TraceInteractionArea
  (params (Trace :type Boolean))
  (if Trace
    (if (Variables|Default|GetIsTracingInteracionArea)
      (Default|ToggleFocus (Variables|Default|GetFocusedInteractionArea) false))
    (bind _asbp_interaction_area_master (Utilities|Casting|CastToBP_InteractionArea_Master (Variables|Default|GetFocusedActor)))
    (if (Default|CanFocus _asbp_interaction_area_master (Components|GetOwner))
      (bind _output_get (Variables|Default|SetFocusedInteractionArea _asbp_interaction_area_master))
      (Default|ToggleFocus _output_get true)
      (Variables|Default|SetIsTracingInteracionArea true)
      (else
        (if (Variables|Default|GetIsTracingInteracionArea) :!label _label
          (Variables|Default|SetIsTracingInteracionArea false)
          (Default|ToggleFocus (Variables|Default|GetFocusedInteractionArea) false)
          (Variables|Default|SetFocusedActor 0)
          (Variables|Default|SetFocusedInteractionArea 0))))
    (else
      (goto _label))))

(fn ResetTrace
  (Variables|Default|SetFocusedActor 0))