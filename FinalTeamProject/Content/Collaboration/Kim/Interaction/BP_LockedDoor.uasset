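; BP_LockedDoor is an interactable door that starts locked and ignores interaction until its OpenDoor event unlocks it.
; BeginPlay runs Init, shows the closed prompt on the interaction widget and sets the lock flag, which gates InteractWithDoor.
; OpenDoor clears the flag and switches the widget text and GMMain outline to open.
; Focus changes toggle the door's custom depth and have GMMain pick the locked or open outline.
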(event Custom|OpenDoor
  (Variables|Default|SetNowLocked false)
  (bind _aswb_interaction_2 (Utilities|Casting|CastToWB_Interaction_2 (UserInterface|GetWidget (Variables|Default|GetWidget))))
  (Default|SetOpenTxt _aswb_interaction_2)
  (Default|SetOpenOutline (Variables|Default|GetGM%20Main)))

(event EventBeginPlay
  (CallFunction|Init)
  (Default|SetCloseTxt (Variables|Default|GetWB%20Interaction%202))
  (Variables|Default|SetNowLocked true))

(event Collision|EventActorBeginOverlap
  (params (OtherActor :type Actor%20Object%20Reference))
  (|CallParentFunction OtherActor) ; This node is disabled and will not be called.\nDrag off pins to build functionality.
)

(event EventTick
  (params (DeltaSeconds :type Float%20%28single-precision%29))
  (|CallParentFunction DeltaSeconds) ; This node is disabled and will not be called.\nDrag off pins to build functionality.
)

(event EventInterfaceToggleFocus
  (params (Focus :type Boolean))
  (bind _gm_main (Variables|Default|GetGM%20Main))
  (if (Variables|Default|GetNowLocked)
    (Default|SetLockOutline _gm_main)
    (else
      (Default|SetOpenOutline _gm_main)))
  (Rendering|SetRenderCustomDepth (Variables|Default|GetDoor) Focus))

(event EventInterfaceInteract
  (if (not (Variables|Default|GetNowLocked))
    (CallFunction|InteractwithDoor)))

(fn ConstructionScript
  (|CallParentFunction))