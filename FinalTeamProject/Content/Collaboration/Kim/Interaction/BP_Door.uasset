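; BP_Door is an interactable sliding door with a widget showing a Korean E-key prompt to open it.
; BeginPlay caches the prompt widget and GM_Main game mode.
; Interface focus events call the game mode's SetOpenOutline and toggle custom depth on the door mesh for highlighting.
; Each interact flips a toggle that plays or reverses a timeline, lerping the door's relative Y location; an alternative yaw-rotation node is left unconnected.
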(event Custom|InteractWithDoor
  (Variables|Default|SetInteractToggle (not (Variables|Default|GetInteractToggle)))
  (if (Variables|Default|GetInteractToggle)
    (bind _doorfloat (Timeline|Timeline Play)
      (:Update
        (Transformation|SetRelativeLocation (Variables|Default|GetDoor) (Math|Vector|MakeVector 0.0 (Math|Float|Lerp -5e+01 5e+01 _doorfloat) 0.0) false false)))
    (else
      (Timeline|Timeline Reverse))))

(event Custom|Init
  (Utilities|FlowControl|Sequence
    (:then_0
      (bind _aswb_interaction_2 (Utilities|Casting|CastToWB_Interaction_2 (UserInterface|GetWidget (Variables|Default|GetWidget))))
      (Variables|Default|SetWB%20Interaction%202 _aswb_interaction_2))
    (:then_1
      (bind _asgm_main (Utilities|Casting|CastToGM_Main (Game|GetGameMode)))
      (Variables|Default|SetGM%20Main _asgm_main))))

(event EventBeginPlay
  (CallFunction|Init)
  (Default|SetTxt (Variables|Default|GetWB%20Interaction%202) "E키를 눌러 문을 엽니다."))

(event Collision|EventActorBeginOverlap
  (params (OtherActor :type Actor%20Object%20Reference)))

(event EventTick
  (params (DeltaSeconds :type Float%20%28single-precision%29)))

(event EventInterfaceToggleFocus
  (params (Focus :type Boolean))
  (Default|SetOpenOutline (Variables|Default|GetGM%20Main))
  (Rendering|SetRenderCustomDepth (Variables|Default|GetDoor) Focus))

(event EventInterfaceInteract
  (CallFunction|InteractwithDoor))

(fn ConstructionScript)