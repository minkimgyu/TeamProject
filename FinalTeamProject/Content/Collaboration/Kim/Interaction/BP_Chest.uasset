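; BP_Chest is an interactable chest actor that opens its inventory as a container through GM_Main.
; On BeginPlay it caches the game mode and its WB_Interaction_2 widget, then sets that widget's open-chest prompt text.
; Interface focus events toggle custom depth on the top and bottom boxes for highlighting.
; Interacting marks it open and passes its InventorySystem and itself to GM_Main's ShowContainer; CloseChest only clears the open flag.
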(event Custom|OpenChest
  (Variables|Default|SetNowOpen true)
  (Default|ShowContainer (Variables|Default|GetGM%20Main) (Variables|Default|GetInventorySystem) self))

(event Custom|CloseChest
  (Variables|Default|SetNowOpen false))

(event EventBeginPlay
  (Utilities|FlowControl|Sequence
    (:then_0
      (bind _asgm_main (Utilities|Casting|CastToGM_Main (Game|GetGameMode)))
      (Variables|Default|SetGM%20Main _asgm_main))
    (:then_1
      (bind _aswb_interaction_2 (Utilities|Casting|CastToWB_Interaction_2 (UserInterface|GetWidget (Variables|Default|GetWidget))))
      (Variables|Default|SetWB%20Interaction%202 _aswb_interaction_2))
    (:then_2
      (Default|SetOpenChestTxt (Variables|Default|GetWB%20Interaction%202)))))

(event Collision|EventActorBeginOverlap
  (params (OtherActor :type Actor%20Object%20Reference)))

(event EventTick
  (params (DeltaSeconds :type Float%20%28single-precision%29)))

(event EventInterfaceToggleFocus
  (params (Focus :type Boolean))
  (Rendering|SetRenderCustomDepth (Variables|Default|GetTopBox) Focus)
  (Rendering|SetRenderCustomDepth (Variables|Default|GetBottomBox) Focus))

(event EventInterfaceInteract
  (CallFunction|OpenChest))

(event EventResetInteractionTrace)

(fn ConstructionScript)